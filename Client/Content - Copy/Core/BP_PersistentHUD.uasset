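; Persistent HUD actor that puts the main menu widget on screen when play begins.
; BeginPlay creates the widget from MainMenuClass, adds it to the viewport and switches input to UI only, focused on it.
; The ToggleMenu action branches on the widget's visibility, but as written the test re-applies Visible or Collapsed to a menu already in that state, so neither flips.
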(event EventBeginPlay
  (bind _returnvalue (UserInterface|CreateWidget (Variables|Default|GetMainMenuClass)))
  (bind _output_get (Variables|Default|SetMainMenuWidget _returnvalue))
  (UserInterface|Viewport|AddtoViewport _output_get 0)
  (Input|SetInputModeUIOnly 0 _output_get "DoNotLock" false))

(event Collision|EventActorBeginOverlap
  (params (OtherActor :type Actor%20Object%20Reference)))

(event EventTick
  (params (DeltaSeconds :type Float%20%28single-precision%29)))

(event Input|ActionEvents|InputActionToggleMenu
  (params (Key :type Key%20Structure :default "None"))
  (bind _mainmenuwidget (Variables|Default|GetMainMenuWidget))
  (:Pressed
    (if (Utilities|IsValid _mainmenuwidget)
      (if (> (Widget|GetVisibility _mainmenuwidget) 0)
        (Widget|SetVisibility _mainmenuwidget "Collapsed")
        (else
          (Widget|SetVisibility _mainmenuwidget "Visible"))))))

(fn ConstructionScript)