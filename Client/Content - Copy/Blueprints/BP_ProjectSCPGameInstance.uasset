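; Game instance Blueprint for ProjectSCP that holds the game mode list and a shared global menu.
; On Init it rebuilds GameModes from every row of the DT_GameModes data table, then selects the first entry as CurrentGameMode.
; InitGlobalMenu creates WBP_GlobalMenu and adds it at a high viewport Z-order, only when no valid instance already exists.
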(event EventInit
  (CallFunction|UpdateGameModes)
  (CallFunction|InitCurrentGameMode))

(fn UpdateGameModes
  (Utilities|Array|Clear (Variables|Default|GetGameModes))
  (bind _outrownames (DataTable|GetDataTableRowNames "/Game/Core/DT_GameModes.DT_GameModes"))
  (for _array_element _outrownames
    (bind _returnvalue (Utilities|GetDataTableRow "/Game/Core/DT_GameModes.DT_GameModes" _array_element)
      (:then
        (Utilities|Array|Add (Variables|Default|GetGameModes) _returnvalue)))))

(fn InitCurrentGameMode
  (if (> (Utilities|Array|Length (Variables|Default|GetGameModes)) 0)
    (bind _output_get (Variables|Default|SetCurrentModeIndex 0))
    (Variables|Default|SetCurrentGameMode (Utilities|Array|Get(acopy) (Variables|Default|GetGameModes) _output_get))))

(fn InitGlobalMenu
  (if (not (Utilities|IsValid (Variables|Default|GetGlobalMenuRef)))
    (bind _returnvalue (UserInterface|CreateWidget "/Game/UI/WBP_GlobalMenu.WBP_GlobalMenu_C"))
    (bind _output_get (Variables|Default|SetGlobalMenuRef _returnvalue))
    (UserInterface|Viewport|AddtoViewport _output_get 99)
    (return _output_get)))