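; Game instance Blueprint for ProjectSCP that runs startup setup for game-wide systems when the game initializes.
; On Init it creates and stores the global menu widget, then calls init steps for mods, game modes, saving and online.
; Mod setup drives a mod manager subsystem to scan and store the installed mod list.
; The game mode, save and online steps are empty stubs.
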(event EventInit
  (CallFunction|InitGlobalMenu)
  (Utilities|InitModManager)
  (CallFunction|InitGameModeManager)
  (CallFunction|InitSaveSystem)
  (CallFunction|InitOnlineSubSystem))

(event Custom|ScanForMods)

(fn InitGlobalMenu
  (bind _returnvalue (UserInterface|CreateWidget "/Game/Core/UI/WBP_GlobalMenu.WBP_GlobalMenu_C"))
  (Variables|Default|SetGlobalMenuWidgetRef _returnvalue))

(fn InitGameModeManager)

(fn InitOnlineSubSystem)

(fn InitSaveSystem)