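; BP_ProjectSCPGameInstance is the game instance for ProjectSCP, holding the list of available game modes and the currently selected one.
; On Init it reads every row of the DT_GameModes data table into the GameModes array.
; If any rows are found, it selects the first entry by setting CurrentModeIndex and CurrentGameMode.
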(event EventInit
  (bind _outrownames (DataTable|GetDataTableRowNames "/Game/Core/DT_GameModes.DT_GameModes"))
  (for _array_element _outrownames
    (bind _returnvalue (Utilities|GetDataTableRow "/Game/Core/DT_GameModes.DT_GameModes" _array_element)
      (:then
        (Utilities|Array|Add (Variables|Default|GetGameModes) _returnvalue))))
  (if (> (Utilities|Array|Length (Variables|Default|GetGameModes)) 0)
    (bind _output_get (Variables|Default|SetCurrentModeIndex 0))
    (Variables|Default|SetCurrentGameMode (Utilities|Array|Get(acopy) (Variables|Default|GetGameModes) _output_get))))